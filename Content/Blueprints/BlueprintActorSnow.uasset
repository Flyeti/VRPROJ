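; Snow-covered actor whose layered mesh material animates its snow through the Sharpness parameter and reacts to trace interaction.
; BeginPlay creates a dynamic material instance, then after a short delay plays a timeline that drives Sharpness.
; Tick restarts that timeline from the start whenever the actor has non-zero velocity.
; Trace handlers tint the mesh on hit and activation, restoring ColorActor when the trace leaves.
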(event Custom|Snow
  (bind _newtrack_0 (Timeline|Timeline_0 Play)
    (:Update
      (Rendering|Material|SetScalarParameterValue (stale EventBeginPlay _returnvalue) "Sharpness" _newtrack_0 :!class /Script/Engine.MaterialInstanceDynamic))))

(event EventBeginPlay
  (bind _returnvalue (Rendering|Material|CreateDynamicMaterialInstance (Variables|Character|GetMesh) 0 "/Game/Materials/SeveralLayersBP.SeveralLayersBP" "None" :!class /Script/Engine.PrimitiveComponent))
  (Rendering|Material|SetScalarParameterValue _returnvalue "Sharpness" 5.0 :!class /Script/Engine.MaterialInstanceDynamic)
  (Utilities|FlowControl|Delay 1.0)
  (CallFunction|Snow))

(event Collision|EventActorBeginOverlap
  (params (OtherActor :type Actor%20Object%20Reference)))

(event EventTick
  (params (DeltaSeconds :type Float%20%28single-precision%29))
  (if (not (Math|Vector|Equal(Vector) (Transformation|GetVelocity) "0, 0, 0" 0.0001))
    (bind _newtrack_0 (Timeline|Timeline_0 PlayFromStart)
      (:Update
        (Rendering|Material|SetScalarParameterValue (stale EventBeginPlay _returnvalue) "Sharpness" _newtrack_0 :!class /Script/Engine.MaterialInstanceDynamic)))))

(fn ConstructionScript)

(fn TraceActivateDown
  (params (Hit :type Hit%20Result%20Structure) (Instigator :type Pawn%20Object%20Reference))
  (Rendering|Material|SetVectorParameterValueonMaterials (Variables|Character|GetMesh) "Color" "1.000000,0.000000,0.000000")
  (return false))

(fn TraceActivateUp
  (params (Hit :type Hit%20Result%20Structure) (Instigator :type Pawn%20Object%20Reference))
  (Rendering|Material|SetVectorParameterValueonMaterials (Variables|Character|GetMesh) "Color" "1.000000,0.300000,0.000000")
  (return false))

(fn TraceHitComponent
  (params (Hit%20%20%20%20%20%20%20%20 :type Hit%20Result%20Structure) (Component :type Primitive%20Component%20Object%20Reference))
  (return false))

(fn TraceHitObject
  (params (Hit :type Hit%20Result%20Structure))
  (Rendering|Material|SetVectorParameterValueonMaterials (Variables|Character|GetMesh) "Color" "1.000000,0.300000, 0")
  (return false))

(fn TraceLeaveObject
  (params (Hit :type Hit%20Result%20Structure))
  (Rendering|Material|SetVectorParameterValueonMaterials (Variables|Character|GetMesh) "Color" (Variables|Default|GetColorActor))
  (return false))

(fn TraceLevelComponent
  (params (Hit :type Hit%20Result%20Structure) (Component :type Primitive%20Component%20Object%20Reference))
  (return false))

(fn TraceMove
  (params (Hit :type Hit%20Result%20Structure%20%28by%20ref%29))
  (return false))